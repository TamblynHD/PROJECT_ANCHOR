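; Main room exit door that ends the game when the player presses E inside its trigger.
; Overlapping Trigger8 shows a prompt and enables input; leaving reverses both.
; E alternates between playing and stopping a timeline that sets the door mesh's yaw.
; The timeline's Update also runs the delayed ending, which shows the end-level widget and then quits the game.
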(event OnComponentBeginOverlap(Trigger8)
  (params (OverlappedComponent :type Primitive%20Component%20Object%20Reference) (OtherActor :type Actor%20Object%20Reference) (OtherComp :type Primitive%20Component%20Object%20Reference) (OtherBodyIndex :type Integer) (bFromSweep :type Boolean) (SweepResult :type Hit%20Result%20Structure%20%28by%20ref%29))
  (Rendering|SetVisibility (Variables|Default|GetPress%20E%20to%20end%20game) true false)
  (Input|EnableInput (Game|GetPlayerController 0)))

(event OnComponentEndOverlap(Trigger8)
  (params (OverlappedComponent :type Primitive%20Component%20Object%20Reference) (OtherActor :type Actor%20Object%20Reference) (OtherComp :type Primitive%20Component%20Object%20Reference) (OtherBodyIndex :type Integer))
  (Rendering|SetVisibility (Variables|Default|GetPress%20E%20to%20end%20game) false false)
  (Input|DisableInput (Game|GetPlayerController 0)))

(event Input|KeyboardEvents|E
  (params (Key :type Key%20Structure))
  (:Pressed
    (if (Variables|Default|GetDoor%20Open/Close)
      (Variables|Default|SetDoor%20Open/Close false)
      (bind _newtrack_0 (Timeline|MainDoor_Open Play)
        (:Update
          (Transformation|SetWorldRotation (Variables|Debug|GetStaticMeshComponent) (Math|Rotator|MakeRotator 0.0 0.0 _newtrack_0) false false)
          (Utilities|FlowControl|Delay 5.5)
          (bind _returnvalue (UserInterface|CreateWidget "/Game/Cut_Scenes/End_Level_Widget.End_Level_Widget_C"))
          (UserInterface|Viewport|AddtoViewport _returnvalue 0)
          (Utilities|FlowControl|Delay 3.0)
          (Game|QuitGame 0 "Quit" false)))
      (else
        (Variables|Default|SetDoor%20Open/Close true)
        (Timeline|MainDoor_Open Stop)))))

(fn ConstructionScript)